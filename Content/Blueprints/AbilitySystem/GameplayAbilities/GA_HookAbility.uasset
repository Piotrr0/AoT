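; Gameplay ability that fires and releases left and right hook projectiles in response to gameplay events.
; On activation it starts four parallel WaitGameplayEvent listeners, one for fire and one for release on each side, and never ends itself.
; Firing sets the gear socket tag, calculates spawn and end locations, then spawns a BP_Hook stored for that side.
; Release events call HookReleased on that side's stored hook if still valid.
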(event `self.K2_ActivateAbility`
  (`|ExecutionSequence`
    (:`then_0`
      (`AbilityTask_WaitGameplayEvent.WaitGameplayEvent` (struct :`TagName` "Events.LeftHookFired") null
        (:`EventReceived`
          (set `self.bLeftHookFired` true)
          (set `self.HookGearTag` (struct :`TagName` "CombatSocket.LeftGear"))
          (`self.FireHook`))))
    (:`then_1`
      (`AbilityTask_WaitGameplayEvent.WaitGameplayEvent` (struct :`TagName` "Events.RightHookFired") null
        (:`EventReceived`
          (set `self.bRightHookFired` true)
          (set `self.HookGearTag` (struct :`TagName` "CombatSocket.RightGear"))
          (`self.FireHook`))))
    (:`then_2`
      (`AbilityTask_WaitGameplayEvent.WaitGameplayEvent` (struct :`TagName` "Events.LeftHookReleased") null
        (:`EventReceived`
          (bind _lefthookprojectile (`self.LeftHookProjectile`)
            (:`then`
              (`HookProjectile.HookReleased` _lefthookprojectile))
            (:`else`)))))
    (:`then_3`
      (`AbilityTask_WaitGameplayEvent.WaitGameplayEvent` (struct :`TagName` "Events.RightHookReleased") null
        (:`EventReceived`
          (bind _righthookprojectile (`self.RightHookProjectile`)
            (:`then`
              (`HookProjectile.HookReleased` _righthookprojectile))
            (:`else`)))))))

(fn `FireHook`
  (locals (SpawnedProjectile :type "/Game/Blueprints/Actor/BP_Hook Object Reference"))
  (`self.CalculateHookSpawnAndEndLocation` (`self.HookGearTag`))
  (bind _returnvalue (`self.SpawnProjectile` (`self.HookSpawnLocation`) (`KismetMathLibrary.MakeRotFromX` (`self.HookEndLocation`))))
  (bind _asbp_hook (cast `/Game/Blueprints/Actor/BP_Hook` _returnvalue))
  (set `local.SpawnedProjectile` _asbp_hook)
  (if (`BlueprintGameplayTagLibrary.MatchesTag` (`self.HookGearTag`) (struct :`TagName` "CombatSocket.LeftGear") true)
    (set `self.LeftHookProjectile` (`local.SpawnedProjectile`))
    (else
      (set `self.RightHookProjectile` (`local.SpawnedProjectile`)))))