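; Hook projectile actor that can be pulled back to the combat socket it was fired from on the player.
; A lifetime timer started at BeginPlay calls PrematureReturn.
; ReturntoOwner runs once, deactivating projectile movement and using a timeline to lerp from the release point to player 0's live FireSocket location.
; When the timeline finishes, the hook destroys itself and fires the returned-to-owner delegate with its socket.
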(event `self.ReceiveBeginPlay`
  (`KismetSystemLibrary.K2_SetTimerDelegate` (delegate `CustomEvent`) (`self.HookLifeTime`)))

(event `CustomEvent`
  (`self.PrematureReturn`))

(event `self.ReturnToOwner`
  (if (not (`self.bReturning`))
    (set `self.bReturning` true)
    (`ActorComponent.SetActive` (`self.ProjectileMovement`) false false)
    (set `self.LocationBeforeReleased` (`self.K2_GetActorLocation`))
    (bind (_direction _returntimeline) (`Timeline|Timeline`)
      (:`Update`
        (bind _returnvalue (message `CombatInterface.GetCombatSocketLocation` (`GameplayStatics.GetPlayerPawn` 0) (`self.FireSocket`)))
        (`self.K2_SetActorLocation` (`KismetMathLibrary.VLerp` (`self.LocationBeforeReleased`) _returnvalue _returntimeline)))
      (:`Finished`
        (`self.K2_DestroyActor`)
        (`self.HookRetunedToOwnerDelegate` (`self.FireSocket`))))))

(fn `UserConstructionScript`)